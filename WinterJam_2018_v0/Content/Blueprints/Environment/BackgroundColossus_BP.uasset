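; BackgroundColossus_BP is a background environment actor that sways back and forth along world X and Z through code-driven movement.
; Each Tick moves it by a counter times per-axis rates, while the counter ramps between positive and negative MovementInterval, easing each reversal.
; MovementOffset seeds the counter at BeginPlay to set the starting phase.
; Steps ignore delta time, so motion depends on frame rate.
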(event `self.ReceiveBeginPlay`
  ;[1 1 1] Begin
  (set `self.MovementCounter` (`self.MovementOffset`)))

(event `self.ReceiveTick`
  (params (DeltaSeconds :type "Float (single-precision)"))
  ;[0.03694 0 1] Movement Animation
  (if (`self.isMovingRight`)
    (if (>= (`self.MovementCounter`) (`self.MovementInterval`))
      (set `self.MovementCounter` (+ (`self.MovementCounter`) 1))
      (set `self.isMovingRight` false)
      (else
        (`self.K2_SetActorLocation` (`KismetMathLibrary.MakeVector` (+ (.x (`self.K2_GetActorLocation`)) (* (`KismetMathLibrary.Conv_IntToDouble` (`self.MovementCounter`)) (`self.MovementRate_X`))) (.y (`self.K2_GetActorLocation`)) (+ (.z (`self.K2_GetActorLocation`)) (* (`KismetMathLibrary.Conv_IntToDouble` (`self.MovementCounter`)) (`self.MovementRate_Z`)))))
        (set `self.MovementCounter` (+ (`self.MovementCounter`) 1))))
    (elif (<= (`self.MovementCounter`) (* (`self.MovementInterval`) -1))
      (set `self.MovementCounter` (+ (`self.MovementCounter`) 1))
      (set `self.isMovingRight` true)
      (else
        (`self.K2_SetActorLocation` (`KismetMathLibrary.MakeVector` (+ (.x (`self.K2_GetActorLocation`)) (* (`KismetMathLibrary.Conv_IntToDouble` (`self.MovementCounter`)) (`self.MovementRate_X`))) (.y (`self.K2_GetActorLocation`)) (+ (.z (`self.K2_GetActorLocation`)) (* (`KismetMathLibrary.Conv_IntToDouble` (`self.MovementCounter`)) (`self.MovementRate_Z`)))))
        (set `self.MovementCounter` (- (`self.MovementCounter`) 1))))))

(fn `UserConstructionScript`)