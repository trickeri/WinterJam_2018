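; Colossus head intro actor that sways back and forth along a diagonal in the X-Z plane.
; Each Tick offsets its location by a counter times per-axis rates, while a direction flag ramps that counter between positive and negative interval limits.
; The counter acts as a velocity, easing the swing at each turn without a timeline, and the motion is frame-rate dependent because delta time is unused.
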(event `self.ReceiveTick`
  (params (DeltaSeconds :type "Float (single-precision)"))
  ;[0.03694 0 1] Movement Animation
  (if (`self.isMovingRight`)
    (if (>= (`self.MovementCounter`) (`self.MovementInterval`))
      (set `self.MovementCounter` (+ (`self.MovementCounter`) 1))
      (set `self.isMovingRight` false)
      (else
        (`self.K2_SetActorLocation` (`KismetMathLibrary.MakeVector` (+ (.x (`self.K2_GetActorLocation`)) (* (`KismetMathLibrary.Conv_IntToDouble` (`self.MovementCounter`)) (`self.MovementRate_X`))) (.y (`self.K2_GetActorLocation`)) (+ (.z (`self.K2_GetActorLocation`)) (* (`KismetMathLibrary.Conv_IntToDouble` (`self.MovementCounter`)) (`self.MovementRate_Z`)))))
        (set `self.MovementCounter` (+ (`self.MovementCounter`) 1))))
    (elif (<= (`self.MovementCounter`) (* (`self.MovementInterval`) -1))
      (set `self.MovementCounter` (+ (`self.MovementCounter`) 1))
      (set `self.isMovingRight` true)
      (else
        (`self.K2_SetActorLocation` (`KismetMathLibrary.MakeVector` (+ (.x (`self.K2_GetActorLocation`)) (* (`KismetMathLibrary.Conv_IntToDouble` (`self.MovementCounter`)) (`self.MovementRate_X`))) (.y (`self.K2_GetActorLocation`)) (+ (.z (`self.K2_GetActorLocation`)) (* (`KismetMathLibrary.Conv_IntToDouble` (`self.MovementCounter`)) (`self.MovementRate_Z`)))))
        (set `self.MovementCounter` (- (`self.MovementCounter`) 1))))))

(fn `UserConstructionScript`)