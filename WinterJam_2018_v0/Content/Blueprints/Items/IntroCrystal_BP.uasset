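; IntroCrystal_BP is a one-shot trigger item that starts the intro cinematic when the player character enters its box.
; It polls the box's overlapping actors every Tick rather than binding an overlap event.
; On detection it plays the PlayerFalls level sequence, calls IntroCinematicTimer on Platforming_GameMode, then destroys itself.
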(event `self.ReceiveTick`
  (params (DeltaSeconds :type "Float (single-precision)"))
  (if (!= (`KismetArrayLibrary.Array_Length` (`PrimitiveComponent.GetOverlappingActors` (`self.Box`) "/Game/Blueprints/Player/PlayerCharacter_BP.PlayerCharacter_BP_C")) 0)
    (bind _outactor (`LevelSequencePlayer.CreateLevelSequencePlayer` "/Game/Sequences/PlayerFalls.PlayerFalls"))
    (`MovieSceneSequencePlayer.Play` (`LevelSequenceActor.SequencePlayer` _outactor))
    (bind _asplatforming_game_mode (cast `/Game/Blueprints/General/Platforming_GameMode` (`GameplayStatics.GetGameMode`)))
    (`/Game/Blueprints/General/Platforming_GameMode.IntroCinematicTimer` _asplatforming_game_mode)
    (`self.K2_DestroyActor`)))

(fn `UserConstructionScript`)