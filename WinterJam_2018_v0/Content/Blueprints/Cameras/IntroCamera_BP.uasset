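; IntroCamera_BP is a camera actor that scrolls along the world X axis to follow the player, apparently for an intro sequence.
; Each Tick, it checks two screen-padding components for an overlapping PlayerCharacter_BP and moves at a fixed, frame-rate-independent speed, toward +X for the right one, otherwise -X for the left.
; The overlap debug print, empty AdjustForPlayer event and disconnected screen-projection nodes are unfinished leftovers.
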(event `AdjustForPlayer`)

(event `self.ReceiveTick`
  (params (DeltaSeconds :type "Float (single-precision)"))
  (bind _returnvalue (* DeltaSeconds 50.0))
  (if (!= (`KismetArrayLibrary.Array_Length` (`PrimitiveComponent.GetOverlappingActors` (`self.PlayerRightScreenPadding`) "/Game/Blueprints/Player/PlayerCharacter_BP.PlayerCharacter_BP_C")) 0)
    (`self.K2_SetActorLocation` (`KismetMathLibrary.MakeVector` (+ (.x (`self.K2_GetActorLocation`)) _returnvalue) (.y (`self.K2_GetActorLocation`)) (.z (`self.K2_GetActorLocation`))))
    (elif (!= (`KismetArrayLibrary.Array_Length` (`PrimitiveComponent.GetOverlappingActors` (`self.PlayerLeftScreenPadding`) "/Game/Blueprints/Player/PlayerCharacter_BP.PlayerCharacter_BP_C")) 0)
      (`self.K2_SetActorLocation` (`KismetMathLibrary.MakeVector` (- (.x (`self.K2_GetActorLocation`)) _returnvalue) (.y (`self.K2_GetActorLocation`)) (.z (`self.K2_GetActorLocation`)))))))

(event `self.ReceiveActorBeginOverlap`
  (params (OtherActor :type "Actor Object Reference"))
  (if (== (`GameplayStatics.GetObjectClass` OtherActor) null)
    (`KismetSystemLibrary.PrintString` "Hello")))

(fn `UserConstructionScript`)