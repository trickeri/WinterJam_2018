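; Side-scrolling platformer camera that follows the player pawn along X with Y locked to zero.
; Each Tick, TrackPlayer holds X inside a dead zone, otherwise lerps toward the offset player position, four times faster beyond a maximum margin.
; Z tracking looks unfinished: its lerp has zero alpha and starts from the camera's X.
; Debug prints remain, and an older padding-volume nudge approach is left unwired.
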(event `AdjustForPlayer`)

(event `self.ReceiveTick`
  (params (DeltaSeconds :type "Float (single-precision)"))
  (`self.TrackPlayer` DeltaSeconds))

(event `self.ReceiveActorBeginOverlap`
  (params (OtherActor :type "Actor Object Reference"))
  (if (== (`GameplayStatics.GetObjectClass` OtherActor) null)
    (`KismetSystemLibrary.PrintString` "Hello")))

(fn `TrackPlayer`
  (params (deltaTime :type "Float (double-precision)"))
  (locals (targetX :type "Float (double-precision)") (targetY :type "Float (double-precision)") (targetZ :type "Float (double-precision)"))
  (bind _xmaximummargin (`self.xMaximumMargin`))
  (bind _x (.x (`self.K2_GetActorLocation` (`GameplayStatics.GetPlayerPawn` 0))))
  (`|ExecutionSequence`
    (:`then_0`
      (bind _output_get (set `self.xDelta` (`KismetMathLibrary.Abs` (- (.x (`self.K2_GetActorLocation`)) (+ _x (`self.xCameraOffset`))))))
      (bind _returnvalue (> _output_get (`self.xDeadZoneHalfWidth`)))
      (if (and _returnvalue (> _output_get _xmaximummargin))
        (bind _output_get_2 (set `local.targetX` (`KismetMathLibrary.Lerp` (.x (`self.K2_GetActorLocation`)) (+ _x (`self.xCameraOffset`)) (* (`self.xSmooth`) deltaTime 4.0))))
        (`KismetSystemLibrary.PrintString` (`KismetStringLibrary.Conv_DoubleToString` _output_get_2))
        (elif (and _returnvalue (< _output_get _xmaximummargin))
          (bind _output_get_3 (set `local.targetX` (`KismetMathLibrary.Lerp` (.x (`self.K2_GetActorLocation`)) (+ _x (`self.xCameraOffset`)) (* (`self.xSmooth`) deltaTime))))
          (`KismetSystemLibrary.PrintString` (`KismetStringLibrary.Conv_DoubleToString` _output_get_3))
          (else
            (set `local.targetX` (.x (`self.K2_GetActorLocation`)))))))
    (:`then_1`
      (bind _output_get_4 (set `self.zDelta` (`KismetMathLibrary.Abs` (- (.z (`self.K2_GetActorLocation`)) (+ (.z (`self.K2_GetActorLocation` (`GameplayStatics.GetPlayerPawn` 0))) (`self.zCameraOffset`))))))
      (if (and (> _output_get_4 (`self.zDeadZoneHalfHeight`)) (> _output_get_4 (`self.zMaximumMargin`)))
        (set `local.targetZ` (`KismetMathLibrary.Lerp` (.x (`self.K2_GetActorLocation`)) (+ 0.0 (`self.zCameraOffset`)) (* (`self.zSmooth`) 0.0 (`self.zDelta`))))))
    (:`then_2`
      (`self.K2_SetActorLocation` (`KismetMathLibrary.MakeVector` (`local.targetX`) 0.0 (`local.targetZ`))))))

(fn `UserConstructionScript`)